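; BP_Pipe is a self-propagating scoring obstacle, apparently for a Flappy Bird-style Paper2D game.
; When an overlap with PaperSprite1 ends, it spawns the next pipe a fixed distance along X at a random height.
; If the player's BP_MyCharacter has not been hit, it adds a point, plays a score sound and destroys itself after a short delay.
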(event `self.PaperSprite1.OnComponentEndOverlap`
  (params (OverlappedComponent :type "PrimitiveComponent Object Reference") (OtherActor :type "Actor Object Reference") (OtherComp :type "PrimitiveComponent Object Reference") (OtherBodyIndex :type Integer))
  (`|SpawnActorFromClass` "BP_Pipe_C" (`KismetMathLibrary.Conv_VectorToTransform` (`KismetMathLibrary.MakeVector` (+ (.x (`SceneComponent.K2_GetComponentLocation` (`self.Root`))) 600.0) (.y (`SceneComponent.K2_GetComponentLocation` (`self.Root`))) (`KismetMathLibrary.RandomFloatInRange` -100.0 50.0))) "Undefined" "OverrideRootScale")
  (bind _asbp_my_character (cast `/Game/Bluprint/BP_MyCharacter` (`GameplayStatics.GetPlayerCharacter` 0)))
  (if (not (`/Game/Bluprint/BP_MyCharacter.Hit` _asbp_my_character))
    (set `/Game/Bluprint/BP_MyCharacter.Score` (+ (`/Game/Bluprint/BP_MyCharacter.Score` _asbp_my_character) 1) _asbp_my_character)
    (`GameplayStatics.PlaySoundAtLocation` "/Game/Art/Audio/SFX_Score_01_Cue.SFX_Score_01_Cue")
    (`KismetSystemLibrary.Delay` 2.0)
    (`self.K2_DestroyActor`)))

(fn `UserConstructionScript`)