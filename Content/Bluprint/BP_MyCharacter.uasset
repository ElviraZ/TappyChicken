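; Player character for a Flappy Bird-style game: a flipbook chicken that drifts along X and flaps upward on touch.
; Each flap launches it and pitches the sprite using its previously recorded position.
; A capsule hit or a failed per-tick screen-Y bounds check sets Hit and calls Die.
; Die repositions the character, runs the BestScore save logic and opens the game-over widget with UI-only input.
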(event `self.ReceiveTick`
  (params (DeltaSeconds :type "Float (single-precision)"))
  (if (not (`self.Hit`))
    (`self.OnViewPort`)
    (`self.K2_AddActorWorldOffset` (0.8 0.0 0.0))))

(event `InputTouch`
  (params (Location :type "Vector Structure") (FingerIndex :type "ETouchIndex Enum"))
  (:`Pressed`
    (`GameplayStatics.PlaySoundAtLocation` "/Game/Art/Audio/SFX_FlapWing_Cue.SFX_FlapWing_Cue")
    (if (not (`self.Hit`))
      (`self.Rot`)
      (`self.LaunchCharacter` (0.0 0.0 250.0)))))

(event `self.CapsuleComponent.OnComponentHit`
  (params (HitComponent :type "PrimitiveComponent Object Reference") (OtherActor :type "Actor Object Reference") (OtherComp :type "PrimitiveComponent Object Reference") (NormalImpulse :type "Vector Structure") (Hit :type "HitResult Structure (by ref)"))
  (`GameplayStatics.PlaySoundAtLocation` "/Game/Art/Audio/SFX_HitGround_01_Cue.SFX_HitGround_01_Cue")
  (set `self.Hit` true)
  (`PaperFlipbookComponent.SetFlipbook` (`self.Sprite`) "/Game/Art/Flip/T_TappyChicken_02.T_TappyChicken_02")
  (`self.Die`))

(event `Die`
  (`self.K2_AddActorWorldOffset` (0.0 200.0 0.0))
  (`self.K2_SetActorRotation` (struct :`Pitch` -90.0))
  (`self.Save`)
  (`WidgetBlueprintLibrary.SetInputMode_UIOnlyEx` (`GameplayStatics.GetPlayerController` 0))
  (bind _returnvalue (`|CreateWidget` "/Game/UMG/W_GameOver.W_GameOver_C"))
  (`UserWidget.AddToViewport` _returnvalue 0))

(fn `OnViewPort`
  (bind (_x _y) (`KismetMathLibrary.BreakVector2D` (`PlayerController.ProjectWorldLocationToScreen` (`GameplayStatics.GetPlayerController` 0) (`SceneComponent.K2_GetComponentLocation` (`self.CapsuleComponent`)) false)))
  (if (not (and (> _y 0.0) (> (`KismetMathLibrary.BreakVector2D` (`WidgetLayoutLibrary.GetViewportSize`)) _y)))
    (set `self.Hit` true)
    (`self.Die`)))

(fn `Rot`
  (bind _returnvalue (`SceneComponent.K2_GetComponentLocation` (`self.CapsuleComponent`)))
  (set `self.Start` _returnvalue)
  (`SceneComponent.K2_SetRelativeRotation` (`self.Sprite`) (`KismetMathLibrary.NegateRotator` (`KismetMathLibrary.MakeRotator` 0.0 (.pitch (`KismetMathLibrary.FindLookAtRotation` (`self.Start`) (`self.Target`))))) false false)
  (set `self.Target` _returnvalue))

(fn `Save`
  (bind _saveref (`self.SaveRef`))
  (bind _returnvalue (`GameplayStatics.CreateSaveGameObject` "/Game/Bluprint/BP_SaveGame.BP_SaveGame_C"))
  (set `self.SaveRef` _returnvalue)
  (bind _returnvalue_2 (`GameplayStatics.DoesSaveGameExist` "SaveGame"))
  (if _returnvalue_2
    (bind _returnvalue_3 (`GameplayStatics.LoadGameFromSlot` ""))
    (bind _asbp_save_game (cast `/Game/Bluprint/BP_SaveGame` _returnvalue_3))
    (if (not (> (`/Game/Bluprint/BP_SaveGame.BestScore` _asbp_save_game) (`self.Score`)))
      (set `/Game/Bluprint/BP_SaveGame.BestScore` (`self.Score`) _saveref)
      (`GameplayStatics.SaveGameToSlot` _saveref "SaveGame"))
    (else
      (set `/Game/Bluprint/BP_SaveGame.BestScore` (`self.Score`) (`self.SaveRef`)))))

(fn `UserConstructionScript`)